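; BP_MoveActor is an actor that slides its sphere back and forth while all BP_ChangeColor actors in the level share a valid color.
; On BeginPlay it binds to each box's color dispatcher, then rechecks the match on each event to start or clear a looping timer running Update Move.
; MoveSphere ping-pongs the sphere along local X; separate helpers, uncalled here, include a minute/second counter that prints and nudges the actor.
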(event Custom|커스텀이벤트_0
  (기본/디폴트|IsSameColor))

(event EventBeginPlay
  (Utilities|FlowControl|Sequence
    (:then_0
      (bind _outactors (Actor|GetAllActorsOfClass "/MyPlugin/BluePrints/MoveActor/BP_ChangeColor.BP_ChangeColor_C"))
      (bind _output_get (Variables|Default|SetColor%20Box _outactors))
      (for _array_element _output_get
        (EventDispatchers|BindEventtoEventDispatcherColor _array_element (delegate Custom|커스텀이벤트_0))))))

(fn ConstructionScript)

(fn CountTimer
  (params (B :type Float%20%28single-precision%29))
  (bind _returnvalue (* 1.0 B))
  (Variables|CountTimer|SetTotalDist (+ _returnvalue (Variables|CountTimer|GetTotalDist)))
  (bind _returnvalue_2 (CountTimer|IF))
  (bind _returnvalue_3 (CountTimer|IF2))
  (if (not (Utilities|Enum|Equal(Enum) (Utilities|String|Append _returnvalue_2 "분 " _returnvalue_3 "초") (Variables|CountTimer|Getcomparison)))
    (bind _output_get (Variables|CountTimer|Setcomparison (Utilities|String|Append _returnvalue_2 "분 " _returnvalue_3 "초")))
    (Development|PrintString _output_get true true "(R=0.000000,G=0.660000,B=1.000000,A=1.000000)" 3.0)
    (Transformation|AddActorLocalOffset (Math|Vector|MakeVector (* 1e+01 _returnvalue) 0.0 0.0) false false)))

(fn PrintHello
  (Development|PrintString "Hello BP_Move Actor"))

(fn GetAPB
  (params (A :type Float%20%28single-precision%29) (B :type Float%20%28single-precision%29))
  (return (+ A B)))

(fn MoveSphere
  (params (MoveSpeed :type Float%20%28single-precision%29))
  (bind _sphere (Variables|Default|GetSphere))
  (if (Variables|Default|GetisRight)
    (bind _result (Math|Float|NegateFloat MoveSpeed)
      (:%20%20
        (Transformation|AddLocalOffset _sphere (Math|Vector|MakeVector _result 0.0 0.0) false false)
        (if (> 0.0 (.x (Variables|/Script/Engine.SceneComponent|GetRelativeLocation (Variables|Default|GetSphere))))
          (Variables|Default|SetisRight false))))
    (else
      (Transformation|AddLocalOffset _sphere (Math|Vector|MakeVector MoveSpeed 0.0 0.0) false false)
      (if (> (.x (Variables|/Script/Engine.SceneComponent|GetRelativeLocation (Variables|Default|GetSphere))) 2e+02)
        (Variables|Default|SetisRight true)))))

(fn IF
  (bind _totaldist (Variables|CountTimer|GetTotalDist))
  (bind _returnvalue (Math|Float|Truncate _totaldist))
  (bind _returnvalue_2 (/ _returnvalue 60))
  (if (< _returnvalue_2 10)
    (return (Utilities|String|Append "0" (Utilities|String|ToString(Integer) _returnvalue_2)))
    (else
      (return (Utilities|String|ToString(Integer) _returnvalue_2)))))

(fn IF2
  (bind _totaldist (Variables|CountTimer|GetTotalDist))
  (bind _returnvalue (Math|Float|Truncate _totaldist))
  (bind _returnvalue_2 (Math|Integer|%(Integer) _returnvalue 60))
  (if (< _returnvalue_2 10)
    (return (Utilities|String|Append "0" (Utilities|String|ToString(Integer) _returnvalue_2)))
    (else
      (return (Utilities|String|ToString(Integer) _returnvalue_2)))))

(fn CheckBox
  (bind _color_box (Variables|Default|GetColor%20Box))
  (bind _output (Utilities|Array|Get(acopy) _color_box))
  (bind _color (Variables|/MyPlugin/BluePrints/MoveActor/BP_ChangeColor.BP_ChangeColor_C|GetColor _output))
  (for _array_element _color_box
    (if (not (and (Utilities|Enum|Equal(Enum) (Variables|/MyPlugin/BluePrints/MoveActor/BP_ChangeColor.BP_ChangeColor_C|GetColor _array_element) _color) (Utilities|Enum|NotEqual(Enum) _color "NewEnumerator2")))
      (return false)))
  (return true))

(fn IsSameColor
  (bind _issamebox (기본/디폴트|CheckBox))
  (if _issamebox
    (Utilities|Time|SetTimerbyFunctionName 0 "Update Move" 0.01 true)
    (else
      (Utilities|Time|ClearTimerbyFunctionName 0 "Update Move"))))

(fn UpdateMove
  (CallFunction|MoveSphere 3.0))