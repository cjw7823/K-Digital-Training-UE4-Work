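; BP_ChangeColor is a collision-learning actor with a cube that changes color when BP_MyCharacter begins overlapping it.
; The overlap switches on the Color variable, applies the matching red or blue vertex-color view-mode material, then flips Color for the next overlap.
; Any other Color value is treated like Blue.
; Every branch then fires the color event dispatcher so bound listeners can react.
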(event OnComponentBeginOverlap(Cube)
  (params (OverlappedComponent :type Primitive%20Component%20Object%20Reference) (OtherActor :type Actor%20Object%20Reference) (OtherComp :type Primitive%20Component%20Object%20Reference) (OtherBodyIndex :type Integer) (bFromSweep :type Boolean) (SweepResult :type Hit%20Result%20Structure%20%28by%20ref%29))
  (bind _cube (Variables|Default|GetCube))
  (Utilities|Casting|CastToBP_MyCharacter OtherActor)
  (switch Utilities|FlowControl|Switch|SwitchonEnum_Color (Variables|Default|GetColor)
    (:NewEnumerator0
      (Rendering|Material|SetMaterial _cube 0 "/Engine/EngineDebugMaterials/VertexColorViewMode_RedOnly.VertexColorViewMode_RedOnly")
      (Variables|Default|SetColor "NewEnumerator1")
      (Default|CallEventDispatcherColor))
    (:NewEnumerator1
      (Rendering|Material|SetMaterial _cube 0 "/Engine/EngineDebugMaterials/VertexColorViewMode_BlueOnly.VertexColorViewMode_BlueOnly")
      (Variables|Default|SetColor "NewEnumerator0")
      (Default|CallEventDispatcherColor))
    (:NewEnumerator2
      (Rendering|Material|SetMaterial _cube 0 "/Engine/EngineDebugMaterials/VertexColorViewMode_BlueOnly.VertexColorViewMode_BlueOnly")
      (Variables|Default|SetColor "NewEnumerator0")
      (Default|CallEventDispatcherColor))))

(fn ConstructionScript)