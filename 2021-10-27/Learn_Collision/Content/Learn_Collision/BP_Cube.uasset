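; BP_Cube is a collision-learning cube that prints elapsed time since BeginPlay while something overlaps it.
; Two looping timers accumulate time continuously and check the overlap flag, printing a Korean minutes-and-seconds string only when it changes.
; Overlap events set that flag and cast to BP_MyHUD without using it.
; Material-swap functions for BP_MyCharacter overlaps exist but are not called here.
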(event OnComponentEndOverlap(Cube)
  (params (OverlappedComponent :type Primitive%20Component%20Object%20Reference) (OtherActor :type Actor%20Object%20Reference) (OtherComp :type Primitive%20Component%20Object%20Reference) (OtherBodyIndex :type Integer))
  (Variables|Default|SetOn%20Overlap false)
  (Utilities|Casting|CastToBP_MyHUD (HUD|GetHUD (Game|GetPlayerController 0))))

(event OnComponentBeginOverlap(Cube)
  (params (OverlappedComponent :type Primitive%20Component%20Object%20Reference) (OtherActor :type Actor%20Object%20Reference) (OtherComp :type Primitive%20Component%20Object%20Reference) (OtherBodyIndex :type Integer) (bFromSweep :type Boolean) (SweepResult :type Hit%20Result%20Structure%20%28by%20ref%29))
  (Variables|Default|SetOn%20Overlap true)
  (Utilities|Casting|CastToBP_MyHUD (HUD|GetHUD (Game|GetPlayerController 0))))

(event EventBeginPlay
  (Utilities|Time|SetTimerbyFunctionName 0 "AddTime" 0.01 true)
  (Utilities|Time|SetTimerbyFunctionName 0 "CountTimer" 0.01 true))

(fn ConstructionScript)

(fn BeginOverlapChangeColor
  (params (Other%20Actor :type Object%20Object%20Reference))
  (Utilities|Casting|CastToBP_MyCharacter Other%20Actor)
  (Rendering|Material|SetMaterial (Variables|Default|GetCube) 0 "/Game/StarterContent/Blueprints/Assets/M_LightStage_Skybox_HDRI.M_LightStage_Skybox_HDRI"))

(fn EndOverlapChangeColor
  (params (Other%20Actor :type Object%20Object%20Reference))
  (Utilities|Casting|CastToBP_MyCharacter Other%20Actor)
  (Rendering|Material|SetMaterial (Variables|Default|GetCube) 0 "/Game/StarterContent/Materials/M_Brick_Clay_New.M_Brick_Clay_New"))

(fn CountTimer
  (bind _total_ds (Variables|Default|GetTotal%20DS))
  (bind _hour (CountTimer|Min _total_ds))
  (bind _min (CountTimer|Second _total_ds))
  (bind _returnvalue (Utilities|String|ToString(Integer) _hour))
  (bind _returnvalue_2 (Utilities|String|ToString(Integer) _min))
  (bind _returnvalue_3 (Utilities|String|Append _returnvalue "분 " _returnvalue_2 "초"))
  (if (Variables|Default|GetOn%20Overlap)
    (if (Utilities|Enum|NotEqual(Enum) _returnvalue_3 (Variables|Default|Getcomparison))
      (bind _output_get (Variables|Default|Setcomparison _returnvalue_3))
      (Development|PrintString _output_get))))

(fn Min
  (params (Delta%20Second :type Float%20%28single-precision%29))
  (return (Math|Float|Truncate (/ Delta%20Second 6e+01))))

(fn Second
  (params (Delta%20Second :type Float%20%28single-precision%29))
  (return (Math|Float|Truncate (Math|Float|%(Float) Delta%20Second 6e+01))))

(fn AddTime
  (Variables|Default|SetTotal%20DS (+ (Variables|Default|GetTotal%20DS) 0.01)))