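; BP_MoveRect is a collision-learning actor that moves its Sphere component around a rectangular path in the XY plane.
; BeginPlay starts a fast looping timer on MoveRect, which switches on MoveType to call one of four directional move functions.
; Each function offsets the Sphere's relative location by Speed and, past the DestPos bound on its axis, sets MoveType to the next side, cycling right, top, left, bottom.
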(event EventBeginPlay
  (Utilities|Time|SetTimerbyFunctionName 0 "MoveRect" 0.01 true))

(fn ConstructionScript)

(fn MoveRight
  (params (Speed :type Float%20%28single-precision%29))
  (Transformation|AddRelativeLocation (Variables|Default|GetSphere) (Math|Vector|MakeVector Speed 0.0 0.0) false false)
  (if (> (.x (Variables|/Script/Engine.SceneComponent|GetRelativeLocation (Variables|Default|GetSphere))) (Variables|Default|GetDestPos))
    (Variables|Default|SetMoveType "NewEnumerator5")))

(fn MoveLeft
  (params (Speed :type Float%20%28single-precision%29))
  (bind _result (Math|Float|NegateFloat Speed)
    (:%20%20
      (Transformation|AddRelativeLocation (Variables|Default|GetSphere) (Math|Vector|MakeVector _result 0.0 0.0) false false)
      (if (> (stale _result_2) (.x (Variables|/Script/Engine.SceneComponent|GetRelativeLocation (Variables|Default|GetSphere))))
        (bind _result_2 (Math|Float|NegateFloat (Variables|Default|GetDestPos))
          (:%20%20
            (Variables|Default|SetMoveType "NewEnumerator6")))))))

(fn MoveBot
  (params (Speed :type Float%20%28single-precision%29))
  (bind _result (Math|Float|NegateFloat Speed)
    (:%20%20
      (Transformation|AddRelativeLocation (Variables|Default|GetSphere) (Math|Vector|MakeVector 0.0 _result 0.0) false false)
      (if (> (stale _result_2) (.y (Variables|/Script/Engine.SceneComponent|GetRelativeLocation (Variables|Default|GetSphere))))
        (bind _result_2 (Math|Float|NegateFloat (Variables|Default|GetDestPos))
          (:%20%20
            (Variables|Default|SetMoveType "NewEnumerator0")))))))

(fn MoveTop
  (params (Speed :type Float%20%28single-precision%29))
  (Transformation|AddRelativeLocation (Variables|Default|GetSphere) (Math|Vector|MakeVector 0.0 Speed 0.0) false false)
  (if (> (.y (Variables|/Script/Engine.SceneComponent|GetRelativeLocation (Variables|Default|GetSphere))) (Variables|Default|GetDestPos))
    (Variables|Default|SetMoveType "NewEnumerator1")))

(fn MoveRect
  (bind _speed (Variables|Default|GetSpeed))
  (switch Utilities|FlowControl|Switch|SwitchonEn_MoveType (Variables|Default|GetMoveType)
    (:NewEnumerator0
      (CallFunction|MoveRight _speed))
    (:NewEnumerator1
      (CallFunction|MoveLeft _speed))
    (:NewEnumerator5
      (CallFunction|MoveTop _speed))
    (:NewEnumerator6
      (CallFunction|MoveBot _speed))))