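; HUD Blueprint that creates and displays HUDWidget2 and feeds it the level's countdown, coin counts, score, menu and pick-up guide.
; A looping one-second timer subtracts elapsed seconds from LimitTime and formats clamped minutes and seconds with table-sourced unit text.
; SetCoin and SetTextScore cache values and defer updates by timer if the widget is not yet valid; only the score path keeps retrying.
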(event EventBeginPlay
  (bind _returnvalue (UserInterface|CreateWidget "/Game/FirstGame/Widget/HUDWidget2.HUDWidget2_C"))
  (bind _output_get (Variables|Default|SetHudWidget _returnvalue))
  (UserInterface|Viewport|AddtoViewport _output_get 0)
  (Utilities|Time|SetTimerbyFunctionName 0 "PrintTime" 1.0 true)
  (Input|SetInputModeGameOnly (Game|GetPlayerController 0)))

(fn ConstructionScript)

(fn PrintTime
  (Variables|Default|SetTotal%20Second (+ (Variables|Default|GetTotal%20Second) 1.0))
  (Variables|/Game/FirstGame/Widget/HUDWidget2.HUDWidget2_C|SetTime (Variables|Default|GetHudWidget) (Utilities|Text|ToText(String) (Utilities|String|Append (Timer|InttoStr00 (Timer|Min (Math|Float|Clamp(Float) (- (Variables|Default|GetLimit%20Time) (Variables|Default|GetTotal%20Second)) 0.0 5e+02))) (Utilities|String|ToString(Text) (CallFunction|GetTableText "text05")) (Timer|InttoStr00 (Timer|Second (Math|Float|Clamp(Float) (- (Variables|Default|GetLimit%20Time) (Variables|Default|GetTotal%20Second)) 0.0 5e+02))) (Utilities|String|ToString(Text) (CallFunction|GetTableText "text06"))))))

(fn Min
  (params (Delta%20Second :type Float%20%28single-precision%29))
  (return (Math|Float|Truncate (/ Delta%20Second 6e+01))))

(fn Second
  (params (Delta%20Second :type Float%20%28single-precision%29))
  (return (Math|Float|Truncate (Math|Float|%(Float) Delta%20Second 6e+01))))

(fn InttoStr00
  (params (Int :type Integer))
  (if (> Int 10)
    (return (Utilities|String|ToString(Integer) Int))
    (else
      (return (Utilities|String|Append "0" (Utilities|String|ToString(Integer) Int))))))

(fn SetCoin
  (params (Hidden :type Integer) (Max :type Integer))
  (Variables|Default|SetHidden Hidden)
  (Variables|Default|SetMax Max)
  (Utilities|IsValid (Variables|Default|GetHudWidget)
    (:Is%20Valid
      (CountCoin|UpdateSetCoin))
    (:Is%20Not%20Valid
      (Utilities|Time|SetTimerbyFunctionName 0 "UpdateSetCoin" 0.1))))

(fn UpdateSetCoin
  (bind _hudwidget (Variables|Default|GetHudWidget))
  (Utilities|FlowControl|Sequence
    (:then_0
      (Variables|/Game/FirstGame/Widget/HUDWidget2.HUDWidget2_C|SetHidden%20Coin%20Count _hudwidget (Utilities|Text|ToText(Integer) (Variables|Default|GetHidden))))
    (:then_1
      (Variables|/Game/FirstGame/Widget/HUDWidget2.HUDWidget2_C|SetMax%20Coin%20Count _hudwidget (Utilities|Text|ToText(Integer) (Variables|Default|GetMax))))))

(fn ShowMenu
  (Default|ShowMenu (Variables|Default|GetHudWidget)))

(fn SetTextScore
  (params (Score :type Integer))
  (Variables|Default|SetBackupScore Score)
  (Utilities|IsValid (Variables|Default|GetHudWidget)
    (:Is%20Valid
      (Default|SetTextScore (Variables|Default|GetHudWidget) Score))
    (:Is%20Not%20Valid
      (Utilities|Time|SetTimerbyFunctionName 0 "UpdateSTS" 0.1))))

(fn UpdateSTS
  (bind _hudwidget (Variables|Default|GetHudWidget))
  (Utilities|IsValid _hudwidget
    (:Is%20Valid
      (Default|SetTextScore _hudwidget (Variables|Default|GetBackupScore)))
    (:Is%20Not%20Valid
      (Utilities|Time|SetTimerbyFunctionName 0 "UpdateSTS" 0.1))))

(fn UpdatePickUpGuidePosition
  (params (WorldLocation :type Vector))
  (Default|UpdateGuidePosition (Variables|Default|GetHudWidget) WorldLocation))

(fn HidePickUpGuide
  (Default|HideGuidePosition (Variables|Default|GetHudWidget)))