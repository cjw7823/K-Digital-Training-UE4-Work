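; BP_FirstGameMode is a game mode that tracks the player's score and shows it on the HUD.
; The score lives in BP_FirstGameInstance, and BeginPlay pushes the stored value to BP_MyHUD2 through the first player controller.
; IncScore raises that stored score by a fixed amount and refreshes the HUD text.
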(event EventBeginPlay
  (bind _asbp_first_game_instance (Utilities|Casting|CastToBP_FirstGameInstance (Game|GetGameInstance)))
  (bind _asbp_my_hud2 (Utilities|Casting|CastToBP_MyHUD2 (HUD|GetHUD (Game|GetPlayerController 0))))
  (Default|SetTextScore _asbp_my_hud2 (Variables|/Game/FirstGame/GameMode/BP_FirstGameInstance.BP_FirstGameInstance_C|GetScore _asbp_first_game_instance)))

(fn ConstructionScript)

(fn IncScore
  (bind _asbp_first_game_instance (Utilities|Casting|CastToBP_FirstGameInstance (Game|GetGameInstance)))
  (Default|SetScore _asbp_first_game_instance (+ (Variables|/Game/FirstGame/GameMode/BP_FirstGameInstance.BP_FirstGameInstance_C|GetScore _asbp_first_game_instance) 10))
  (bind _asbp_my_hud2 (Utilities|Casting|CastToBP_MyHUD2 (HUD|GetHUD (Game|GetPlayerController 0))))
  (Default|SetTextScore _asbp_my_hud2 (Variables|/Game/FirstGame/GameMode/BP_FirstGameInstance.BP_FirstGameInstance_C|GetScore _asbp_first_game_instance)))