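; BP_CannonBall is a cannon hazard that tracks the player pawn and repeatedly fires a physics ball at it.
; Tick smoothly turns an Arrow component toward the player, serving as the muzzle transform.
; A looping timer calls DoShoot, which recycles one ball component by resetting it to the Arrow, clearing velocity and applying a forward impulse.
; Hitting a BP_SwatCharacter triggers ragdoll, a knockback impulse, an explosion emitter and audio.
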(event OnComponentHit(ConnonBall)
  (params (HitComponent :type Primitive%20Component%20Object%20Reference) (OtherActor :type Actor%20Object%20Reference) (OtherComp :type Primitive%20Component%20Object%20Reference) (NormalImpulse :type Vector :default "0, 0, 0") (Hit :type Hit%20Result%20Structure%20%28by%20ref%29))
  (bind _asbp_swat_character (Utilities|Casting|CastToBP_SwatCharacter OtherActor))
  (Development|PrintString "Hello")
  (Default|DoRagdoll _asbp_swat_character)
  (Physics|AddImpulse (Variables|/Script/Engine.Character|GetMesh _asbp_swat_character) (* (Math|Vector|GetForwardVector (Math|Rotator|FindLookatRotation (Transformation|GetWorldLocation (Variables|Default|GetConnonBall)) (Transformation|GetWorldLocation (Variables|/Script/Engine.Character|GetMesh _asbp_swat_character)))) 1e+04) "None" false)
  (Effects|SpawnEmitteratLocation "/Game/StarterContent/Particles/P_Explosion.P_Explosion" (Transformation|GetWorldLocation (Variables|/Script/Engine.Character|GetMesh _asbp_swat_character)) "0, 0, 0" "1.000000,1.000000,1.000000" false)
  (Audio|Components|Audio|Play (Variables|Default|GetAudio) 0.0))

(event EventBeginPlay
  (Variables|Default|SetTarget (Game|Player|GetPlayerPawn 0))
  (Utilities|Time|SetTimerbyFunctionName 0 "DoShoot" 1.5 true))

(event EventTick
  (params (DeltaSeconds :type Float%20%28single-precision%29))
  (bind _arrow (Variables|Default|GetArrow))
  (Transformation|SetWorldRotation _arrow (Math|Rotator|Lerp(Rotator) (Transformation|GetWorldRotation _arrow) (Math|Rotator|FindLookatRotation (Transformation|GetWorldLocation _arrow) (Transformation|GetActorLocation (Variables|Default|GetTarget))) 0.1 true) false false))

(fn ConstructionScript)

(fn DoShoot
  (bind _connonball (Variables|Default|GetConnonBall))
  (bind _arrow (Variables|Default|GetArrow))
  (Transformation|SetWorldLocationAndRotation (Variables|Default|GetConnonBall) (Transformation|GetWorldLocation _arrow) (Transformation|GetWorldRotation _arrow) false false)
  (Transformation|SetWorldLocation (Variables|Default|GetConnonBall) (Transformation|GetWorldLocation (Variables|Default|GetArrow)) false false)
  (Class|PrimitiveComponent|SetAllPhysicsLinearVelocity (Variables|Default|GetConnonBall) "0, 0,0.000000" false)
  (Physics|AddImpulse _connonball (* (Math|Vector|GetForwardVector _connonball) 5e+05) "None" false))