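; BP_Sword is a sword actor that can be attached to and detached from a character.
; AttachToChar disables physics and collision on its static mesh, then snaps it to a named socket on the character's mesh, keeping world scale.
; DetachToChar restores collision and physics and releases the mesh in place, without using its Character input.
; The event graph and construction script contain no logic.
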(event EventBeginPlay)

(event Collision|EventActorBeginOverlap
  (params (OtherActor :type Actor%20Object%20Reference)))

(event EventTick
  (params (DeltaSeconds :type Float%20%28single-precision%29)))

(fn ConstructionScript)

(fn AttachtoChar
  (params (Character :type Character%20Object%20Reference))
  (bind _staticmesh (Variables|Default|GetStaticMesh))
  (Physics|SetSimulatePhysics _staticmesh false)
  (Collision|SetCollisionEnabled _staticmesh "NoCollision")
  (bind _returnvalue (Transformation|AttachComponentToComponent _staticmesh (Variables|/Script/Engine.Character|GetMesh Character) (Variables|Default|GetSocket%20Name) "SnapToTarget" "SnapToTarget" "KeepWorld" true))
  (return _returnvalue))

(fn DetachtoChar
  (params (Character :type Character%20Object%20Reference))
  (bind _staticmesh (Variables|Default|GetStaticMesh))
  (Collision|SetCollisionEnabled _staticmesh "QueryAndPhysics")
  (Physics|SetSimulatePhysics _staticmesh true)
  (Transformation|DetachFromComponent _staticmesh "KeepWorld" "KeepWorld" "KeepWorld" true)
  (return true))