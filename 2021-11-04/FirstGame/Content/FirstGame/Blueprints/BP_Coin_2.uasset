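; A collectible coin actor that spins, bobs and disappears when a BP_SwatCharacter overlaps it.
; On pickup it hides itself, fires CoinDestroyed and disables the coin's collision.
; BeginPlay caches the level's BP_Portal actors and starts a looping timer calling MoveCoin, which animates the coin without Tick.
; MoveCoin rotates it and calls CoinUpDown, which flips direction at fixed world-height limits rather than relative to its placed position.
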(event OnComponentBeginOverlap(Coin)
  (params (OverlappedComponent :type Primitive%20Component%20Object%20Reference) (OtherActor :type Actor%20Object%20Reference) (OtherComp :type Primitive%20Component%20Object%20Reference) (OtherBodyIndex :type Integer) (bFromSweep :type Boolean) (SweepResult :type Hit%20Result%20Structure%20%28by%20ref%29))
  ;[1 1 1] 먹으면 사라짐
  (Utilities|Casting|CastToBP_SwatCharacter OtherActor)
  (Rendering|SetActorHiddenInGame true)
  (Default|CallCoinDestroyed)
  (Collision|SetCollisionEnabled (Variables|Default|GetCoin) "NoCollision"))

(event EventBeginPlay
  ;[1 1 1] 모든 코인이 움직임.
  (bind _outactors (Actor|GetAllActorsOfClass "/MyPlugin/BluePrints/Coin/BP_Portal.BP_Portal_C"))
  (Variables|Default|SetPortal _outactors)
  (Utilities|Time|SetTimerbyFunctionName 0 "MoveCoin" 0.02 true))

(fn ConstructionScript)

(fn MoveCoin
  ;[1 1 1] 동전 돌리기
  (Class|Actor|AddActorWorldRotation "0,3.000000, 0")
  (CallFunction|CoinUpDown))

(fn CoinUpDown
  (if (Variables|Default|GetIs%20Top)
    (Transformation|AddActorLocalOffset "0, 0,2.000000" false false)
    (if (>= (.z (Transformation|GetActorLocation)) 1e+02)
      (Variables|Default|SetIs%20Top false))
    (else
      (Transformation|AddActorLocalOffset "0, 0,-2.000000" false false)
      (if (>= 5e+01 (.z (Transformation|GetActorLocation)))
        (Variables|Default|SetIs%20Top true)))))