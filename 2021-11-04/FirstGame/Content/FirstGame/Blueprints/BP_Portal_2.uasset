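; Level-exit portal that activates once every BP_Coin_2 in the level is collected and loads LevelName when BP_MyCharacter overlaps it.
; BeginPlay disables portal collision, gathers the coins and binds to their destroyed events.
; OnHiddenCheck treats hidden coins as collected, showing the portal and enabling collision when none remain visible.
; It also updates the BP_MyHUD2 coin counter and increments the BP_FirstGameMode score.
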(event OnComponentBeginOverlap(Portal)
  (params (OverlappedComponent :type Primitive%20Component%20Object%20Reference) (OtherActor :type Actor%20Object%20Reference) (OtherComp :type Primitive%20Component%20Object%20Reference) (OtherBodyIndex :type Integer) (bFromSweep :type Boolean) (SweepResult :type Hit%20Result%20Structure%20%28by%20ref%29))
  ;[1 1 1] 맵 이동
  (Utilities|Casting|CastToBP_MyCharacter OtherActor)
  (Game|OpenLevel(byName) (Variables|Default|GetLevel%20Name)))

(event EventBeginPlay
  (bind (_hidden _max) (CallFunction|CheckHiddenCoins))
  ;[1 1 1] 모든 코인이 사라지면 포탈 생성
  (Collision|SetCollisionEnabled (Variables|Default|GetPortal) "NoCollision")
  (bind _outactors (Actor|GetAllActorsOfClass "/Game/FirstGame/Blueprints/BP_Coin_2.BP_Coin_2_C"))
  (bind _output_get (Variables|Default|SetCoins _outactors))
  (for _array_element _output_get
    (EventDispatchers|BindEventtoCoinDestroyed _array_element (EventDispatchers|CreateEvent :!event OnHiddenCheck))
    ;[1 1 1] HUDWidget 카운트 초기화
    (bind _asbp_my_hud2 (Utilities|Casting|CastToBP_MyHUD2 (HUD|GetHUD (Game|GetPlayerController 0))))
    (Default|SetCoin _asbp_my_hud2 _hidden _max)))

(fn ConstructionScript)

(fn CheckCoin
  (for _array_element (Variables|Default|GetCoins)
    (if (not (Variables|/Script/Engine.Actor|GetbHidden _array_element))
      (return true)))
  (return false))

(fn OnHiddenCheck
  (bind (_hidden _max) (CallFunction|CheckHiddenCoins))
  (Utilities|FlowControl|Sequence
    (:then_0
      ;[1 1 1] 코인 획득 처리
      (bind _isallhidden (CallFunction|CheckCoin))
      (Rendering|SetActorHiddenInGame _isallhidden)
      (if (not _isallhidden)
        (Collision|SetCollisionEnabled (Variables|Default|GetPortal) "QueryAndPhysics")))
    (:then_1
      ;[1 1 1] UI 카운트 업데이트
      (bind _asbp_my_hud2 (Utilities|Casting|CastToBP_MyHUD2 (HUD|GetHUD (Game|GetPlayerController 0))))
      (Default|SetCoin _asbp_my_hud2 _hidden _max)
      (bind _asbp_first_game_mode (Utilities|Casting|CastToBP_FirstGameMode (Game|GetGameMode)))
      (Default|IncScore _asbp_first_game_mode))))

(fn CheckHiddenCoins
  (bind _coins (Variables|Default|GetCoins))
  (for _array_element _coins
    (if (Variables|/Script/Engine.Actor|GetbHidden _array_element)
      (Math|Integer|IncrementInt (LocalVariables|GetHiddenCoins))))
  (return (LocalVariables|GetHiddenCoins) (Utilities|Array|Length _coins)))