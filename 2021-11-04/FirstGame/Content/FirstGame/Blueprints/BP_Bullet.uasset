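; BP_Bullet is a homing projectile that chases player 0's pawn and knocks down the BP_SwatCharacter it hits.
; BeginPlay starts a looping timer on MoveBullet, which snaps the Sphere toward the target and offsets it forward by Speed without sweeping.
; On hitting a swat character, it triggers ragdoll, applies an impulse to the mesh and destroys itself.
; MoveForward offers smoothed-turn homing but is not called here.
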(event OnComponentHit(Sphere)
  (params (HitComponent :type Primitive%20Component%20Object%20Reference) (OtherActor :type Actor%20Object%20Reference) (OtherComp :type Primitive%20Component%20Object%20Reference) (NormalImpulse :type Vector :default "0, 0, 0") (Hit :type Hit%20Result%20Structure%20%28by%20ref%29))
  (bind _asbp_swat_character (Utilities|Casting|CastToBP_SwatCharacter OtherActor))
  (Default|DoRagdoll _asbp_swat_character)
  (Utilities|Time|ClearTimerbyFunctionName 0 "MoveBullet")
  (Physics|AddImpulse (Variables|/Script/Engine.Character|GetMesh _asbp_swat_character) (* (Math|Vector|GetForwardVector (Math|Rotator|FindLookatRotation (Transformation|GetWorldLocation (Variables|Default|GetSphere)) (Transformation|GetWorldLocation (Variables|/Script/Engine.Character|GetMesh _asbp_swat_character)))) 1e+04) "None" false)
  (Actor|DestroyActor))

(event EventBeginPlay
  ;[1 1 1] 코멘트
  (Variables|Default|SetTarget (Game|Player|GetPlayerPawn 0))
  (Utilities|Time|SetTimerbyFunctionName 0 "MoveBullet" 0.01 true))

(fn ConstructionScript)

(fn MoveForward
  (params (A :type Float%20%28single-precision%29))
  (bind _sphere (Variables|Default|GetSphere))
  (bind _sphere_2 (Variables|Default|GetSphere))
  (Utilities|IsValid (Variables|Default|GetTarget)
    (:Is%20Valid
      (Transformation|SetWorldRotation _sphere (Math|Rotator|Lerp(Rotator) (Transformation|GetWorldRotation _sphere_2) (Math|Rotator|FindLookatRotation (Transformation|GetWorldLocation _sphere_2) (Transformation|GetActorLocation (Variables|Default|GetTarget))) 0.01 true) false false)
      (Transformation|AddWorldOffset _sphere (* (Math|Vector|GetForwardVector _sphere) (* A (Variables|Default|GetSpeed))) false false))))

(fn MoveBullet
  (bind _sphere (Variables|Default|GetSphere))
  (bind _sphere_2 (Variables|Default|GetSphere))
  (Utilities|IsValid (Variables|Default|GetTarget)
    (:Is%20Valid
      (Transformation|SetWorldRotation _sphere_2 (Math|Rotator|FindLookatRotation (Transformation|GetWorldLocation _sphere_2) (Transformation|GetActorLocation (Variables|Default|GetTarget))) false false)
      (Transformation|AddWorldOffset _sphere (* (Math|Vector|GetForwardVector _sphere) (Variables|Default|GetSpeed)) false false))
    (:Is%20Not%20Valid
      (Development|PrintString "Non Target"))))