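; Actor that moves its Cube back and forth along its Spline, matching the spline's rotation as it travels.
; From BeginPlay, a timeline value scaled by spline length sets the cube's local transform, preserving scale.
; When the timeline finishes, IsForward flips and the timeline plays or reverses, creating a ping-pong loop.
; An older distance-stepping approach using MoveToSpline remains disconnected and never runs.
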(event Collision|EventActorBeginOverlap
  (params (OtherActor :type Actor%20Object%20Reference)))

(event EventBeginPlay
  (bind _spline (Variables|Default|GetSpline))
  (bind _cube (Variables|Default|GetCube))
  (if (Variables|Default|GetIsForward) :!label _label
    (bind _value (Timeline|타임라인_0 Play)
      (:Update
        (Transformation|SetRelativeTransform _cube (Math|Transform|MakeTransform (.location (Spline|GetTransformatDistanceAlongSpline _spline (* _value (Spline|GetSplineLength _spline)) "Local" false)) (.rotation (Spline|GetTransformatDistanceAlongSpline _spline (* _value (Spline|GetSplineLength _spline)) "Local" false)) (Variables|/Script/Engine.SceneComponent|GetRelativeScale3D _cube)) false false))
      (:Finished
        (bind _output_get (Variables|Default|SetIsForward (not (stale _output_get))))
        (goto _label)))
    (else
      (Timeline|타임라인_0 Reverse))))

(fn ConstructionScript)

(fn MovetoSpline
  (params (Distance :type Float%20%28single-precision%29))
  (bind _spline (Variables|Default|GetSpline))
  (bind _cube (Variables|Default|GetCube))
  (Transformation|SetRelativeTransform _cube (Math|Transform|MakeTransform (Spline|GetLocationatDistanceAlongSpline _spline Distance "Local") (Spline|GetRotationatDistanceAlongSpline _spline Distance "Local") (Variables|/Script/Engine.SceneComponent|GetRelativeScale3D _cube)) false false))