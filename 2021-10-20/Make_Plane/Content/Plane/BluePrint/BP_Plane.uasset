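; BP_Plane is a plane actor that animates itself in constant motion, with no input or flight logic.
; Each Tick spins the Left and Right components rapidly around their roll axis, like propellers.
; The same Tick pushes the Body component forward along its local X axis while slowly rolling it, with all rates scaled by delta time.
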(event EventTick
  (params (DeltaSeconds :type Float%20%28single-precision%29))
  (Variables|Default|SetSpeed (* DeltaSeconds 5.4e+03))
  (Transformation|AddLocalRotation (Variables|Default|GetLeft) (Math|Rotator|MakeRotator (Variables|Default|GetSpeed) 0.0 0.0) false false)
  (Transformation|AddLocalRotation (Variables|Default|GetRight) (Math|Rotator|MakeRotator (Variables|Default|GetSpeed) 0.0 0.0) false false)
  (Class|SceneComponent|AddLocalTransform (Variables|Default|GetBody) (Math|Transform|MakeTransform (Math|Vector|MakeVector (* 100 (Utilities|Time|GetWorldDeltaSeconds)) 0.0 0.0) "0, 0, 0" "1,1,1") false false)
  (Transformation|AddLocalRotation (Variables|Default|GetBody) (Math|Rotator|MakeRotator (* 50 (Utilities|Time|GetWorldDeltaSeconds)) 0.0 0.0) false false))

(fn ConstructionScript)