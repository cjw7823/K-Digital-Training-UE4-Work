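; BP_MoveRect moves its Sphere component around a rectangular loop in relative X and Y while IsRight is enabled.
; Tick dispatches on MoveType to one of four directional functions, each offsetting the sphere by Speed times delta time.
; Each function switches MoveType once the sphere passes a DestPos-based bound, cycling right, top, left, bottom.
; Go toggles IsRight to start or pause the motion.
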(event EventTick
  (params (DeltaSeconds :type Float%20%28single-precision%29))
  (if (Variables|Default|GetIs%20Right)
    (switch Utilities|FlowControl|Switch|SwitchonEn_MoveType (Variables|Default|GetMoveType)
      (:NewEnumerator0
        (CallFunction|MoveRight DeltaSeconds))
      (:NewEnumerator1
        (CallFunction|MoveLeft DeltaSeconds))
      (:NewEnumerator5
        (CallFunction|MoveTop DeltaSeconds))
      (:NewEnumerator6
        (CallFunction|MoveBot DeltaSeconds)))))

(fn ConstructionScript)

(fn MoveRight
  (params (DeltaSecond :type Float%20%28single-precision%29))
  (Transformation|AddRelativeLocation (Variables|Default|GetSphere) (Math|Vector|MakeVector (* DeltaSecond (Variables|Default|GetSpeed)) 0.0 0.0) false false)
  (if (> (.x (Variables|/Script/Engine.SceneComponent|GetRelativeLocation (Variables|Default|GetSphere))) (Variables|Default|GetDestPos))
    (Variables|Default|SetMoveType "NewEnumerator5")))

(fn MoveLeft
  (params (DeltaSecond :type Float%20%28single-precision%29))
  (bind _result (Math|Float|NegateFloat (* DeltaSecond (Variables|Default|GetSpeed)))
    (:%20%20
      (Transformation|AddRelativeLocation (Variables|Default|GetSphere) (Math|Vector|MakeVector _result 0.0 0.0) false false)
      (if (> (stale _result_2) (.x (Variables|/Script/Engine.SceneComponent|GetRelativeLocation (Variables|Default|GetSphere))))
        (bind _result_2 (Math|Float|NegateFloat (Variables|Default|GetDestPos))
          (:%20%20
            (Variables|Default|SetMoveType "NewEnumerator6")))))))

(fn MoveBot
  (params (Delta%20Second :type Float%20%28single-precision%29))
  (bind _result (Math|Float|NegateFloat (* Delta%20Second (Variables|Default|GetSpeed)))
    (:%20%20
      (Transformation|AddRelativeLocation (Variables|Default|GetSphere) (Math|Vector|MakeVector 0.0 _result 0.0) false false)
      (if (> (stale _result_2) (.y (Variables|/Script/Engine.SceneComponent|GetRelativeLocation (Variables|Default|GetSphere))))
        (bind _result_2 (Math|Float|NegateFloat (Variables|Default|GetDestPos))
          (:%20%20
            (Variables|Default|SetMoveType "NewEnumerator0")))))))

(fn MoveTop
  (params (Delta%20Second :type Float%20%28single-precision%29))
  (Transformation|AddRelativeLocation (Variables|Default|GetSphere) (Math|Vector|MakeVector 0.0 (* Delta%20Second (Variables|Default|GetSpeed)) 0.0) false false)
  (if (> (.y (Variables|/Script/Engine.SceneComponent|GetRelativeLocation (Variables|Default|GetSphere))) (Variables|Default|GetDestPos))
    (Variables|Default|SetMoveType "NewEnumerator1")))

(fn Go
  (Variables|Default|SetIs%20Right (not (Variables|Default|GetIs%20Right))))