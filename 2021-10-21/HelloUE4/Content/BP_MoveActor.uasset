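; Test actor that runs an elapsed-time clock on screen and nudges itself along X.
; Tick feeds CountTimer, which accumulates seconds and builds a zero-padded minutes/seconds string with Korean units via IF and IF2.
; Only when that string changes does it print and apply an X offset scaled by that frame's delta.
; MoveSphere (back-and-forth sphere motion), PrintHello and GetAPB are defined but never called here.
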(event EventTick
  (params (DeltaSeconds :type Float%20%28single-precision%29))
  (CountTimer|CountTimer DeltaSeconds))

(fn ConstructionScript)

(fn CountTimer
  (params (B :type Float%20%28single-precision%29))
  (bind _returnvalue (* 1.0 B))
  (Variables|Default|SetTotalDisk (+ _returnvalue (Variables|Default|GetTotalDisk)))
  (bind _returnvalue_2 (CountTimer|IF))
  (bind _returnvalue_3 (CountTimer|IF2))
  (if (not (Utilities|Enum|Equal(Enum) (Utilities|String|Append _returnvalue_2 "분 " _returnvalue_3 "초") (Variables|Default|Getcomparison)))
    (bind _output_get (Variables|Default|Setcomparison (Utilities|String|Append _returnvalue_2 "분 " _returnvalue_3 "초")))
    (Development|PrintString _output_get true true "(R=0.000000,G=0.660000,B=1.000000,A=1.000000)" 3.0)
    (Transformation|AddActorLocalOffset (Math|Vector|MakeVector (* 1e+01 _returnvalue) 0.0 0.0) false false)))

(fn PrintHello
  (Development|PrintString "Hello"))

(fn GetAPB
  (params (A :type Float%20%28single-precision%29) (B :type Float%20%28single-precision%29))
  (return (+ A B)))

(fn MoveSphere
  (params (A :type Float%20%28single-precision%29))
  (bind _returnvalue (* A 1e+02))
  (bind _sphere (Variables|Default|GetSphere))
  (if (Variables|Default|GetisRight)
    (bind _result (Math|Float|NegateFloat _returnvalue)
      (:%20%20
        (Transformation|AddLocalOffset _sphere (Math|Vector|MakeVector _result 0.0 0.0) false false)
        (if (> 0.0 (.x (Variables|/Script/Engine.SceneComponent|GetRelativeLocation (Variables|Default|GetSphere))))
          (Variables|Default|SetisRight false))))
    (else
      (Transformation|AddLocalOffset _sphere (Math|Vector|MakeVector _returnvalue 0.0 0.0) false false)
      (if (> (.x (Variables|/Script/Engine.SceneComponent|GetRelativeLocation (Variables|Default|GetSphere))) 1e+02)
        (Variables|Default|SetisRight true)))))

(fn IF
  (bind _totaldisk (Variables|Default|GetTotalDisk))
  (bind _returnvalue (Math|Float|Truncate _totaldisk))
  (bind _returnvalue_2 (/ _returnvalue 60))
  (if (< _returnvalue_2 10)
    (return (Utilities|String|Append "0" (Utilities|String|ToString(Integer) _returnvalue_2)))
    (else
      (return (Utilities|String|ToString(Integer) _returnvalue_2)))))

(fn IF2
  (bind _totaldisk (Variables|Default|GetTotalDisk))
  (bind _returnvalue (Math|Float|Truncate _totaldisk))
  (bind _returnvalue_2 (Math|Integer|%(Integer) _returnvalue 60))
  (if (< _returnvalue_2 10)
    (return (Utilities|String|Append "0" (Utilities|String|ToString(Integer) _returnvalue_2)))
    (else
      (return (Utilities|String|ToString(Integer) _returnvalue_2)))))