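; Rotating ball actor that swings its Center component back and forth around the roll axis, with a toggle to start and stop it.
; A timeline drives the roll, and its Finished event flips IsTime to alternate forward and reverse playback.
; Toggle uses IsPlay to choose between Play and Stop.
; MoveLikeTimer, not called in the event graph, offers a delta-time swing that reverses beyond 45 degrees either side.
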(event Custom|Stop
  (Variables|Default|SetIsPlay true)
  (bind _value (Timeline|타임라인_0 Stop)
    (:Update
      (Transformation|SetRelativeRotation (Variables|Default|GetCenter) (Math|Rotator|MakeRotator _value 0.0 0.0) false false))
    (:Finished
      (Variables|Default|SetIs%20Time (not (Variables|Default|GetIs%20Time)))
      (if (Variables|Default|GetIs%20Time)
        (Timeline|타임라인_0 Play)
        (else
          (Timeline|타임라인_0 Reverse))))))

(event Custom|Toggle
  (if (Variables|Default|GetIsPlay)
    (CallFunction|Play)
    (else
      (CallFunction|Stop))))

(event Custom|Play
  (Variables|Default|SetIsPlay false)
  (if (Variables|Default|GetIs%20Time) :!label _label
    (bind _value (Timeline|타임라인_0 Play)
      (:Update
        (Transformation|SetRelativeRotation (Variables|Default|GetCenter) (Math|Rotator|MakeRotator _value 0.0 0.0) false false))
      (:Finished
        (Variables|Default|SetIs%20Time (not (Variables|Default|GetIs%20Time)))
        (goto _label)))
    (else
      (Timeline|타임라인_0 Reverse))))

(fn ConstructionScript)

(fn MoveLikeTimer
  (params (A :type Float%20%28single-precision%29))
  (bind _returnvalue (Utilities|Time|GetWorldDeltaSeconds))
  (bind _center (Variables|Default|GetCenter))
  (bind _returnvalue_2 (* A _returnvalue))
  (if (Variables|Default|GetIs%20Right)
    (bind _result (Math|Float|NegateFloat _returnvalue_2)
      (:%20%20
        (Transformation|AddRelativeRotation _center (Math|Rotator|MakeRotator _result 0.0 0.0) false false)
        (if (> -45.0 (.roll (Variables|/Script/Engine.SceneComponent|GetRelativeRotation (Variables|Default|GetCenter))))
          (Variables|Default|SetIs%20Right false))))
    (else
      (Transformation|AddRelativeRotation _center (Math|Rotator|MakeRotator _returnvalue_2 0.0 0.0) false false)
      (if (> (.roll (Variables|/Script/Engine.SceneComponent|GetRelativeRotation (Variables|Default|GetCenter))) 45.0)
        (Variables|Default|SetIs%20Right true)))))