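; BP_MyPawn is a free-moving pawn that appears to be an input-mapping practice asset, with mouse look and axis-driven movement.
; Movement offsets the actor without sweep along the camera's forward and right vectors, scaled by a Speed value that two actions step within bounds.
; On BeginPlay it spawns a BP_MoveActor, calls its PrintHello, and nudges it up or down with R and F.
; Extra test mappings only print debug strings.
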(event EventBeginPlay
  ;[1 1 1] 접속 인사
  (Development|PrintString "Hello" true true "(R=0.000000,G=0.660000,B=1.000000,A=1.000000)" 6e+01)
  (bind _returnvalue (Game|SpawnActorfromClass "/Game/BP_MoveActor.BP_MoveActor_C" (Math|Transform|MakeTransform "0, 0,200.000000") "Undefined" 0 0))
  (bind _output_get (Variables|Default|SetBP_MoveActor _returnvalue))
  (Default|PrintHello _output_get))

(event Input|ActionEvents|InputActionHelloWorld
  (params (Key :type Key%20Structure :default "None"))
  ;[1 1 1] 액션 매핑
  (:Pressed
    (Development|PrintString "HelloWorld Pressed"))
  (:Released
    (Development|PrintString "HelloWorld Relesed")))

(event Input|ActionEvents|InputActionMoveSpeed
  (params (Key :type Key%20Structure :default "None"))
  ;[1 1 1] 1, 2 키로 속도 조절
  (:Pressed
    (if (> (Variables|Default|GetSpeed) 1e+01)
      (Variables|Default|SetSpeed (+ -1e+01 (Variables|Default|GetSpeed))))))

(event Input|ActionEvents|InputActionMoveSpeed2
  (params (Key :type Key%20Structure :default "None"))
  ;[1 1 1] 1, 2 키로 속도 조절
  (:Pressed
    (if (> 1e+02 (Variables|Default|GetSpeed))
      (Variables|Default|SetSpeed (+ 1e+01 (Variables|Default|GetSpeed))))))

(event Input|AxisEvents|InputAxisAxisTest
  (params (AxisValue :type Float%20%28single-precision%29))
  ;[1 1 1] 축 매핑 [Print to Screen] off
  (Development|PrintString (Utilities|String|Append "axis test" (Utilities|String|ToString(Float) AxisValue)) false))

(event Input|AxisEvents|InputAxisMoveRight
  (params (AxisValue :type Float%20%28single-precision%29))
  ;[1 1 1] w,a,s,d 이동
  (Transformation|AddActorWorldOffset (* (Transformation|GetActorRightVector (Game|GetPlayerCameraManager 0)) (* AxisValue (Variables|Default|GetSpeed)))))

(event Input|AxisEvents|InputAxisLook_UP
  (params (AxisValue :type Float%20%28single-precision%29))
  ;[1 1 1] 마우스 화면 회전
  (Pawn|Input|AddControllerPitchInput AxisValue))

(event Input|AxisEvents|InputAxisLook_Right
  (params (AxisValue :type Float%20%28single-precision%29))
  ;[1 1 1] 마우스 화면 회전
  (Pawn|Input|AddControllerYawInput AxisValue))

(event Input|AxisEvents|InputAxisMoveForward
  (params (AxisValue :type Float%20%28single-precision%29))
  ;[1 1 1] w,a,s,d 이동
  (Transformation|AddActorWorldOffset (* (Transformation|GetActorForwardVector (Game|GetPlayerCameraManager 0)) (* AxisValue (Variables|Default|GetSpeed)))))

(event Input|KeyboardEvents|R
  (params (Key :type Key%20Structure :default "None"))
  (:Pressed
    (Transformation|AddActorWorldOffset (Variables|Default|GetBP_MoveActor) "0.000000, 0,10.000000")))

(event Input|KeyboardEvents|F
  (params (Key :type Key%20Structure :default "None"))
  (:Pressed
    (Transformation|AddActorWorldOffset (Variables|Default|GetBP_MoveActor) "0.000000, 0,-10.000000")))

(fn ConstructionScript)