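; BP_MyPawn is a free-fly spectator-style pawn that spawns and controls a set of moving test actors.
; Axis inputs offset it along the camera's forward, right and up vectors and apply mouse look, while two actions step its speed within limits.
; BeginPlay spawns BP_MoveActor, BP_MoveRect, BP_TimelineActor and BP_RotationBall at fixed transforms.
; One action toggles all four actors' motion states, and R/F nudge the MoveActor vertically.
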(event EventBeginPlay
  ;[1 1 1] 스폰 액터
  (bind _returnvalue (Game|SpawnActorfromClass "/Game/BP_MoveActor.BP_MoveActor_C" (Math|Transform|MakeTransform "0, 0,200.000000") "Undefined" 0 0))
  (Variables|Default|SetBP_MoveActor _returnvalue)
  (bind _returnvalue_2 (Game|SpawnActorfromClass "/Game/BP_MoveRect.BP_MoveRect_C" (Math|Transform|MakeTransform "-690.000000,300.000000,300.000000") "Undefined" 0 0))
  (Variables|Default|SetBP_MoveRect _returnvalue_2)
  (bind _returnvalue_3 (Game|SpawnActorfromClass "/Game/BP_TimelineActor.BP_TimelineActor_C" (Math|Transform|MakeTransform "400.000000,200.000000,300.000000") "Undefined" 0 0))
  (Variables|Default|SetBP_TimelineActor _returnvalue_3)
  (bind _returnvalue_4 (Game|SpawnActorfromClass "/Game/BP_RotationBall.BP_RotationBall_C" (Math|Transform|MakeTransform "400.000000,200.000000,700.000000" "0.000000,90.000000,0.000000") "Undefined" 0 0))
  (Variables|Default|SetBP_RotationBall _returnvalue_4))

(event Input|ActionEvents|InputActionMoveSpeed
  (params (Key :type Key%20Structure :default "None"))
  ;[1 1 1] 카메라 액션
  ;;[1 1 1] 1,2 키로 속도 조절
  (:Pressed
    (if (> (Variables|Default|GetSpeed) 1e+01)
      (Variables|Default|SetSpeed (+ -1e+01 (Variables|Default|GetSpeed))))))

(event Input|ActionEvents|InputActionMoveSpeed2
  (params (Key :type Key%20Structure :default "None"))
  ;[1 1 1] 카메라 액션
  ;;[1 1 1] 1,2 키로 속도 조절
  (:Pressed
    (if (> 1e+02 (Variables|Default|GetSpeed))
      (Variables|Default|SetSpeed (+ 1e+01 (Variables|Default|GetSpeed))))))

(event Input|ActionEvents|InputActionMoveRec
  (params (Key :type Key%20Structure :default "None"))
  (bind _bp_moveactor (Variables|Default|GetBP_MoveActor))
  (bind _bp_moverect (Variables|Default|GetBP_MoveRect))
  ;[1 1 1] Spawned Actor Moving
  (:Pressed
    (Variables|/Game/BP_MoveRect.BP_MoveRect_C|SetIs%20Right _bp_moverect (not (Variables|/Game/BP_MoveRect.BP_MoveRect_C|GetIs%20Right _bp_moverect)))
    (Variables|/Game/BP_MoveActor.BP_MoveActor_C|SetisMove _bp_moveactor (not (Variables|/Game/BP_MoveActor.BP_MoveActor_C|GetisMove _bp_moveactor)))
    (Default|Toggle (Variables|Default|GetBP_TimelineActor))
    (Default|Toggle (Variables|Default|GetBP_RotationBall))))

(event Input|AxisEvents|InputAxisMoveUp
  (params (AxisValue :type Float%20%28single-precision%29))
  ;[1 1 1] 카메라 액션
  ;;[1 1 1] Q,E 이동
  (Transformation|AddActorWorldOffset (* (Transformation|GetActorUpVector (Game|GetPlayerCameraManager 0)) (* AxisValue (Variables|Default|GetSpeed)))))

(event Input|AxisEvents|InputAxisMoveRight
  (params (AxisValue :type Float%20%28single-precision%29))
  ;[1 1 1] 카메라 액션
  ;;[1 1 1] w,a,s,d 이동
  (Transformation|AddActorWorldOffset (* (Transformation|GetActorRightVector (Game|GetPlayerCameraManager 0)) (* AxisValue (Variables|Default|GetSpeed)))))

(event Input|AxisEvents|InputAxisLook_UP
  (params (AxisValue :type Float%20%28single-precision%29))
  ;[1 1 1] 카메라 액션
  ;;[1 1 1] 마우스 화면 회전
  (Pawn|Input|AddControllerPitchInput AxisValue))

(event Input|AxisEvents|InputAxisLook_Right
  (params (AxisValue :type Float%20%28single-precision%29))
  ;[1 1 1] 카메라 액션
  ;;[1 1 1] 마우스 화면 회전
  (Pawn|Input|AddControllerYawInput AxisValue))

(event Input|AxisEvents|InputAxisMoveForward
  (params (AxisValue :type Float%20%28single-precision%29))
  ;[1 1 1] 카메라 액션
  ;;[1 1 1] w,a,s,d 이동
  (Transformation|AddActorWorldOffset (* (Transformation|GetActorForwardVector (Game|GetPlayerCameraManager 0)) (* AxisValue (Variables|Default|GetSpeed)))))

(event Input|KeyboardEvents|R
  (params (Key :type Key%20Structure :default "None"))
  ;[1 1 1] BP_MoveActor Z값 변환
  (:Pressed
    (Transformation|AddActorWorldOffset (Variables|Default|GetBP_MoveActor) "0.000000, 0,10.000000")))

(event Input|KeyboardEvents|F
  (params (Key :type Key%20Structure :default "None"))
  ;[1 1 1] BP_MoveActor Z값 변환
  (:Pressed
    (Transformation|AddActorWorldOffset (Variables|Default|GetBP_MoveActor) "0.000000, 0,-10.000000")))

(fn ConstructionScript)