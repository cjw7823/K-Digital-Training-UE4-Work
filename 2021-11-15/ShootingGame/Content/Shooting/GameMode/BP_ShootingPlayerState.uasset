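; BP_ShootingPlayerState is the player state for the shooting game mode, holding each player's HP and display name.
; AddDamage and AddHeal adjust HP within a clamped range, and SetNameABC sets the name.
; RepNotify functions broadcast event dispatchers when either value changes.
; The HP notify fires an additional HUD dispatcher only when this state belongs to player controller 0, separating local HUD updates from general HP updates.
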(fn ConstructionScript)

(fn AddDamage
  (params (Damage :type Float%20%28single-precision%29))
  (Variables|Default|SetHP (Math|Float|Clamp(Float) (- (Variables|Default|GetHP) Damage) 0.0 1e+02)))

(fn OnRepHP
  (Development|PrintString (Utilities|String|Append "AddDamage CurHP-" (Utilities|String|ToString(Float) (Variables|Default|GetHP))) false false "(R=0.000000,G=0.660000,B=1.000000,A=1.000000)" 2e+01)
  (Default|CallEventDispatcherUpdateHP (Variables|Default|GetHP) 1e+02)
  (if (== self (Variables|/Script/Engine.Controller|GetPlayerState (Game|GetPlayerController 0)))
    (Default|CallEventDispatcherUpdateHPHUD (Variables|Default|GetHP) 1e+02)))

(fn AddHeal
  (params (Heal :type Float%20%28single-precision%29))
  (Variables|Default|SetHP (Math|Float|Clamp(Float) (+ (Variables|Default|GetHP) Heal) 0.0 1e+02)))

(fn SetNameABC
  (params (NickName :type String))
  (Variables|Default|SetName NickName))

(fn OnRepName
  (Default|CallEventDispatcherChangeName (Variables|Default|GetName)))