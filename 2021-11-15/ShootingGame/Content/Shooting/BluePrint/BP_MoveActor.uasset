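; Shooting-folder actor whose Cube component slides back and forth along its local X axis.
; MoveActor acts only with authority, toggling a fast looping timer that starts or stops the motion on each call.
; Each tick of that timer offsets the Cube by a fixed step and flips the IsRight flag when it passes either end of its travel range.
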(event EventMoveActor
  (Networking|SwitchHasAuthority
    (:Authority
      (if (Class|KismetSystemLibrary|TimerExists 0 "UpdateMoveRightLeft")
        (Utilities|Time|ClearTimerbyFunctionName 0 "UpdateMoveRightLeft")
        (else
          (Utilities|Time|SetTimerbyFunctionName 0 "UpdateMoveRightLeft" 0.01 true))))))

(fn ConstructionScript)

(fn UpdateMoveRightLeft
  (if (Variables|Default|GetIsRight)
    (Transformation|AddLocalOffset (Variables|Default|GetCube) (Math|Vector|MakeVector 1e+01 0.0 0.0) false false)
    (if (> (.x (Variables|/Script/Engine.SceneComponent|GetRelativeLocation (Variables|Default|GetCube))) 5e+02)
      (Variables|Default|SetIsRight false))
    (else
      (Transformation|AddLocalOffset (Variables|Default|GetCube) (Math|Vector|MakeVector -1e+01 0.0 0.0) false false)
      (if (> 0.1 (.x (Variables|/Script/Engine.SceneComponent|GetRelativeLocation (Variables|Default|GetCube))))
        (Variables|Default|SetIsRight true)))))