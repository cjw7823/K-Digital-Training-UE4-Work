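; BP_RandomSpawnWeapon scatters random weapon pickups or actors around its own location when play begins.
; It loops a fixed number of times, choosing each weapon from the DT_Weapon row names, with the last two rows excluded from the random pick.
; Each spawn lands on a random navmesh point within a radius, rolled onto its side with random yaw, and receives the row name as WeaponName.
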(event EventBeginPlay
  (bind _outrownames (DataTable|GetDataTableRowNames "/Game/Shooting/Data/DT_Weapon.DT_Weapon"))
  (Variables|Default|SetOut%20Row%20Names _outrownames)
  (for _index (range 0 10)
    (Game|SpawnActorfromClass "/Game/Shooting/BluePrint/BP_Weapon_Auto.BP_Weapon_Auto_C" (Math|Transform|MakeTransform (.RandomLocation (Class|NavigationSystemV1|GetRandomPointinNavigableRadius (Transformation|GetActorLocation) 2e+03 0 0)) (Math|Rotator|MakeRotator 9e+01 0.0 (.Yaw (Math|Rotator|BreakRotator (Math|Random|RandomRotator false)))) "1,1,1") "Undefined" 0 (Utilities|Array|Get(acopy) (Variables|Default|GetOut%20Row%20Names) (Math|Random|RandomInteger (- (Utilities|Array|Length (Variables|Default|GetOut%20Row%20Names)) 2))) 0)))

(fn ConstructionScript)