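; BP_SpawnWeapon is a weapon spawner that creates a random weapon when an actor overlaps it.
; BeginPlay caches the row names of the DT_Weapon data table.
; The OnActorOverlap override calls its parent, then spawns BP_Weapon_Auto at the spawner's location, passing a random name from the first four rows as WeaponName.
; The overlap logic here neither filters the overlapping actor nor limits repeat spawns.
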(event EventBeginPlay
  (bind _outrownames (DataTable|GetDataTableRowNames "/Game/Shooting/Data/DT_Weapon.DT_Weapon"))
  (Variables|Default|SetOut%20Row%20Names _outrownames))

(fn ConstructionScript
  (|CallParentFunction))

(fn OnActorOverlap
  (params (OtherActor :type Actor%20Object%20Reference))
  (|CallParentFunction 0)
  (Game|SpawnActorfromClass "/Game/Shooting/BluePrint/BP_Weapon_Auto.BP_Weapon_Auto_C" (Math|Transform|MakeTransform (Transformation|GetActorLocation) "0, 0, 0" "1,1,1") "Undefined" 0 (Utilities|Array|Get(acopy) (Variables|Default|GetOut%20Row%20Names) (Math|Random|RandomIntegerinRange 0 3)) 0))